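; Enemy pawn that chases and shoots at the first-person character and explodes when killed.
; On sighting via PawnSensing it turns toward the player, moves with AIMoveTo and, if Shoot is set, spawns a projectile with zero impulse.
; Damage lowers Life, but death is checked only on Cube hits, triggering a timed explosion effect and delayed destruction.
; The Shoot cooldown logic is disconnected and never runs.
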(event `self.Cube.OnComponentHit`
  (params (HitComponent :type "PrimitiveComponent Object Reference") (OtherActor :type "Actor Object Reference") (OtherComp :type "PrimitiveComponent Object Reference") (NormalImpulse :type "Vector Structure") (Hit :type "HitResult Structure (by ref)"))
  (if (<= (`self.Life`) 0.0)
    (`|ExecutionSequence`
      (:`then_0`
        (bind _returnvalue (`|SpawnActorFromClass` "/Game/StarterContent/Blueprints/Blueprint_Effect_Explosion.Blueprint_Effect_Explosion_C" (`SceneComponent.K2_GetComponentToWorld` (`self.Cube`)) "Undefined" "OverrideRootScale" null null))
        (`self.SetLifeSpan` _returnvalue (`KismetMathLibrary.Conv_IntToDouble` (`KismetMathLibrary.RandomIntegerInRange` 6 10)))
        (`KismetSystemLibrary.Delay` 1.0)
        (`self.K2_DestroyActor`))
      (:`then_1`
        (`ActorComponent.K2_DestroyComponent` (`self.Cube`))))))

(event `self.ReceiveAnyDamage`
  (params (Damage :type "Float (single-precision)") (DamageType :type "DamageType Object Reference") (InstigatedBy :type "Controller Object Reference") (DamageCauser :type "Actor Object Reference"))
  (set `self.Life` (- (`self.Life`) Damage)))

(event `self.PawnSensing.OnSeePawn`
  (params (Pawn :type "Pawn Object Reference"))
  (bind _asfirst_person_character (cast `/Game/FirstPersonBP/Blueprints/FirstPersonCharacter` Pawn))
  (`|ExecutionSequence`
    (:`then_0`
      (`self.K2_SetActorRotation` (`KismetMathLibrary.FindLookAtRotation` (`self.K2_GetActorLocation`) (`self.K2_GetActorLocation` _asfirst_person_character))))
    (:`then_1`
      (`|AIMoveTo` self (0.0 0.0 0.0) _asfirst_person_character))
    (:`then_2`
      (if (`self.Shoot`)
        (bind _returnvalue (`|SpawnActorFromClass` "/Game/FirstPersonBP/Blueprints/EnemyProjectile.EnemyProjectile_C" (`SceneComponent.K2_GetComponentToWorld` (`self.SpawnShootPoint`)) "AlwaysSpawn" "OverrideRootScale" null null))
        (`PrimitiveComponent.AddImpulse` (`/Game/FirstPersonBP/Blueprints/EnemyProjectile.Sphere` _returnvalue) (0.0 0.0 0.0) "None" false)))))

(fn `UserConstructionScript`)