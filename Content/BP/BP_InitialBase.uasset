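; BP_InitialBase is a trigger actor that lets the first-person player grab a target.
; Any overlap on its Box toggles a GrabAllow flag, with no check on which actor overlaps.
; While allowed, Tick polls the player character's Grab flag, then destroys TargetActor, disables the Box's collision and sets the character's Grabbed flag.
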(event `self.Box.OnComponentBeginOverlap`
  (params (OverlappedComponent :type "PrimitiveComponent Object Reference") (OtherActor :type "Actor Object Reference") (OtherComp :type "PrimitiveComponent Object Reference") (OtherBodyIndex :type Integer) (bFromSweep :type Boolean) (SweepResult :type "HitResult Structure (by ref)"))
  (set `self.GrabAllow` true))

(event `self.Box.OnComponentEndOverlap`
  (params (OverlappedComponent :type "PrimitiveComponent Object Reference") (OtherActor :type "Actor Object Reference") (OtherComp :type "PrimitiveComponent Object Reference") (OtherBodyIndex :type Integer))
  (set `self.GrabAllow` false))

(event `self.ReceiveTick`
  (params (DeltaSeconds :type "Float (single-precision)"))
  (if (`self.GrabAllow`)
    (bind _asfirst_person_character (cast `/Game/FirstPersonBP/Blueprints/FirstPersonCharacter` (`GameplayStatics.GetPlayerCharacter` 0)))
    (if (`/Game/FirstPersonBP/Blueprints/FirstPersonCharacter.Grab` _asfirst_person_character)
      (`|ExecutionSequence`
        (:`then_0`
          (`self.K2_DestroyActor` (`self.TargetActor`))
          (`PrimitiveComponent.SetCollisionEnabled` (`self.Box`) "NoCollision"))
        (:`then_1`
          (set `/Game/FirstPersonBP/Blueprints/FirstPersonCharacter.Grabbed` true _asfirst_person_character))))))

(fn `UserConstructionScript`)